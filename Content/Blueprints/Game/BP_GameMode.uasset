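; BP_GameMode is a game mode Blueprint that relays match start and end to the players' BP_PlayerController instances.
; StartGameBP loops over PlayerControllers and has each create a start-game timer.
; EndGameBP calls EndGameClient with false on the losing controller, then with true on the first other controller found, so only one winner is notified.
; BeginPlay and Tick are empty, and some debug printing is left unconnected.
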(event EventBeginPlay)

(event EventTick
  (params (DeltaSeconds :type Float%20%28single-precision%29)))

(event EventStartGameBP
  (for _array_element (Variables|Default|GetPlayerControllers)
    (bind _asbp_player_controller (Utilities|Casting|CastToBP_PlayerController _array_element))
    (Default|CreateStartGameTimer _asbp_player_controller)))

(event EventEndGameBP
  (params (Looser :type Player%20Controller%20Object%20Reference))
  (bind _asbp_player_controller (Utilities|Casting|CastToBP_PlayerController Looser)
    (:then
      (Default|EndGameClient _asbp_player_controller false))
    (:CastFailed
      _))
  (bind _array_element (Utilities|Array|ForEachLoopwithBreak (Variables|Default|GetPlayerControllers) :!label _label)
    (:LoopBody
      (if (!= _array_element Looser)
        (bind _asbp_player_controller_2 (Utilities|Casting|CastToBP_PlayerController _array_element))
        (Default|EndGameClient _asbp_player_controller_2 true)
        (goto _label Break)))))

(fn ConstructionScript)