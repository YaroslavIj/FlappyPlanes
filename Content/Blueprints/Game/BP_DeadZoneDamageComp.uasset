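; BP_DeadZoneDamageComp is a dead-zone damage component that repeatedly damages a Plane after a short grace period.
; BeginPlay starts a one-shot delay timer, which then starts a looping timer that applies DamagePerTick to the Plane whenever that reference is valid.
; Stop clears both timer handles, cancelling pending or ongoing damage, and Tick is unused.
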(event Custom|StartDamage
  (bind _returnvalue (Utilities|Time|SetTimerbyEvent (delegate Custom|DamageTick) 1.0 true))
  (Variables|Default|SetDamageTickTimer _returnvalue))

(event Custom|DamageTick
  (bind _plane (Variables|Default|GetPlane))
  (Utilities|IsValid _plane
    (:Is%20Valid
      (Class|FlappyPlane|ReceiveDamage _plane (Variables|Default|GetDamagePerTick)))))

(event Custom|Stop
  (Utilities|Time|ClearandInvalidateTimerbyHandle (Variables|Default|GetStartDamageTimer))
  (Utilities|Time|ClearandInvalidateTimerbyHandle (Variables|Default|GetDamageTickTimer)))

(event EventBeginPlay
  (bind _returnvalue (Utilities|Time|SetTimerbyEvent (delegate Custom|StartDamage) 3.0))
  (Variables|Default|SetStartDamageTimer _returnvalue))

(event EventTick
  (params (DeltaSeconds :type Float%20%28single-precision%29)))