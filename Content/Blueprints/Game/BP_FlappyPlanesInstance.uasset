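; BP_FlappyPlanesInstance is the Flappy Planes game instance, reporting results of online login and session operations through on-screen debug prints.
; It handles EOS login, session creation and session join events, printing success or failure for each.
; Session creation also calls the parent implementation, suggesting the session logic lives in the parent class.
; Network error handling is empty, and the nodes opening the menu or listen-server map are disconnected.
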(event EventHandleNetworkError
  (params (FailureType :type ENetworkFailure%20Enum :default "NetDriverAlreadyExists") (bIsServer :type Boolean)))

(event EventOnEOSLoginCompleted
  (params (bWasSuccessful :type Boolean) (Error :type Name :default "None"))
  (if bWasSuccessful
    (Development|PrintString "Login Successful")
    (else
      (Development|PrintString (Utilities|String|Append "Login Error: " (Utilities|String|ToString(Name) Error))))))

(event EventOnCreateSessionCompleted
  (params (SessionName :type Name :default "None") (bWasSuccessful :type Boolean))
  (|CallParentFunction SessionName bWasSuccessful)
  (if bWasSuccessful
    (Development|PrintString (Utilities|String|Append "SessionCreated, Name: " (Utilities|String|ToString(Name) SessionName)))
    (elif (!= SessionName "")
      (Development|PrintString (Utilities|String|ToString(Name) SessionName))
      (else
        (Development|PrintString "CreateSessionFailed")))))

(event EventOnJoinSessionCompletedBP
  (params (bWasSuccessful :type Boolean) (Message :type Name :default "None"))
  (if bWasSuccessful
    (Development|PrintString "JoinSessionSuccesful")
    (else
      (Development|PrintString (Utilities|String|ToString(Name) Message) true true "(R=0.000000,G=0.660000,B=1.000000,A=1.000000)" 1e+01))))