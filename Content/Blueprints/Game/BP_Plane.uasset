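; Plane actor linked to an owning pawn, which forwards its health, fuel and projectile count to the UI.
; Change delegates and OnRep events both update a 3D health widget on the plane and, for locally controlled pawns, fuel and ammo through BP_PlayerController.
; BeginPlay initializes the health widget differently for the first local player's plane than for all others.
; Tick prints a debug plane-to-pawn distance while the pawn has a controller.
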(event Custom|OnHealthChanged_Event
  (params (NewHealth :type Float%20%28single-precision%29))
  (CallFunction|SetHealthonWidget NewHealth))

(event Custom|OnFuelChanged_Event
  (params (NewFuel :type Float%20%28single-precision%29))
  (CallFunction|SetFuelonWidget NewFuel))

(event Custom|OnProjectilesAmountChanged_Event
  (params (NewProjectilesAmount :type Float%20%28single-precision%29))
  (CallFunction|SetProjectilesAmountonWidget NewProjectilesAmount))

(event Custom|SetHealthOnWidget
  (params (NewHealth :type Float%20%28double-precision%29))
  (bind _asbpw_3dhealth (Utilities|Casting|CastToBPW_3DHealth (UserInterface|GetWidget (Variables|Default|GetWidget))))
  (Default|SetHealth _asbpw_3dhealth NewHealth))

(event Custom|SetFuelOnWidget
  (params (NewFuel :type Float%20%28double-precision%29))
  (bind _asbp_pawn (Utilities|Casting|CastToBP_Pawn (Variables|Default|GetPawnOwner)))
  (Utilities|IsValid (Pawn|GetController _asbp_pawn)
    (:Is%20Valid
      (if (Pawn|IsLocalPlayerController (Pawn|GetController _asbp_pawn))
        (bind _asbp_player_controller (Utilities|Casting|CastToBP_PlayerController (Pawn|GetController _asbp_pawn)))
        (Default|SetFuelonWidget _asbp_player_controller NewFuel)))))

(event Custom|SetProjectilesAmountOnWidget
  (params (NewProjectilesAmount :type Float%20%28double-precision%29))
  (bind _asbp_pawn (Utilities|Casting|CastToBP_Pawn (Variables|Default|GetPawnOwner)))
  (Utilities|IsValid (Pawn|GetController _asbp_pawn)
    (:Is%20Valid
      (if (Pawn|IsLocalPlayerController (Pawn|GetController _asbp_pawn))
        (bind _asbp_player_controller (Utilities|Casting|CastToBP_PlayerController (Pawn|GetController _asbp_pawn)))
        (Default|SetProjectilesAmountonWidgt _asbp_player_controller NewProjectilesAmount)))))

(event Custom|CustomEvent
  (Physics|SetSimulatePhysics (Variables|Default|GetPlaneMesh) false))

(event EventBeginPlay
  (bind _pawnowner (Variables|Default|GetPawnOwner))
  (bind _returnvalue (Pawn|GetController _pawnowner))
  (Utilities|FlowControl|Sequence
    (:then_0
      (EventDispatchers|AssignOnHealthChanged (delegate Custom|OnHealthChanged_Event))
      (EventDispatchers|AssignOnFuelChanged (delegate Custom|OnFuelChanged_Event))
      (EventDispatchers|AssignOnProjectilesAmountChanged (delegate Custom|OnProjectilesAmountChanged_Event)))
    (:then_1
      (Utilities|IsValid _pawnowner
        (:Is%20Valid
          (bind _asbpw_3dhealth (Utilities|Casting|CastToBPW_3DHealth (UserInterface|GetWidget (Variables|Default|GetWidget))))
          (Utilities|IsValid _returnvalue
            (:Is%20Valid
              (if (== (Game|GetPlayerController 0) _returnvalue)
                (Default|Init _asbpw_3dhealth false)
                (else
                  (Default|Init _asbpw_3dhealth true))))
            (:Is%20Not%20Valid
              (Default|Init _asbpw_3dhealth true))))))))

(event Collision|EventActorBeginOverlap
  (params (OtherActor :type Actor%20Object%20Reference)))

(event EventOnRepHealth
  (bind _returnvalue (Class|FlappyPlane|GetCurrentHealth))
  (CallFunction|SetHealthonWidget _returnvalue))

(event EventTick
  (params (DeltaSeconds :type Float%20%28single-precision%29))
  (Utilities|IsValid (Pawn|GetController (Variables|Default|GetPawnOwner))
    (:Is%20Valid
      (Development|PrintString (Utilities|String|ToString(Float) (Math|Vector|Distance(Vector) (Transformation|GetActorLocation) (Transformation|GetActorLocation (Variables|Default|GetPawnOwner)))) true true "(R=0.000000,G=0.660000,B=1.000000,A=1.000000)" 0.0))))

(event EventOnRepFuel
  (CallFunction|SetFuelonWidget (Variables|Default|GetFuel)))

(event EventOnRepProjectilesAmount
  (CallFunction|SetProjectilesAmountonWidget (Math|Conversions|ToFloat(Integer) (Variables|Default|GetProjectilesAmount))))

(fn ConstructionScript)