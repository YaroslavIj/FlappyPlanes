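; BP_ParallaxBackground is an actor that creates parallax by moving with the player pawn at a scaled rate.
; Each Tick offsets it by the pawn's movement since the previous frame times SpeedCoef, without sweeping.
; LastCameraLocation stores the pawn's location, not the camera's.
; BeginPlay assigns that variable to itself, so the first offset is measured from its initial value.
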(event EventBeginPlay
  (Utilities|IsValid (Game|Player|GetPlayerPawn 0)
    (:Is%20Valid
      (Variables|Default|SetLastCameraLocation (Variables|Default|GetLastCameraLocation)))))

(event Collision|EventActorBeginOverlap
  (params (OtherActor :type Actor%20Object%20Reference)))

(event EventTick
  (params (DeltaSeconds :type Float%20%28single-precision%29))
  (bind _returnvalue (Game|Player|GetPlayerPawn 0))
  (bind _returnvalue_2 (Transformation|GetActorLocation _returnvalue))
  (Utilities|IsValid _returnvalue
    (:Is%20Valid
      (Transformation|AddActorWorldOffset (* (- _returnvalue_2 (Variables|Default|GetLastCameraLocation)) (Variables|Default|GetSpeedCoef)))
      (Variables|Default|SetLastCameraLocation _returnvalue_2))))

(fn ConstructionScript)