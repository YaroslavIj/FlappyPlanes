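; Parallax background layer that scrolls with the player and tiles itself endlessly along Y.
; Each tick it offsets itself by the pawn's Y/Z movement scaled by SpeedCoef.
; It deprojects a screen corner to its depth to estimate the visible edges, spawning linked, slightly overlapping copies of itself where an edge is uncovered.
; Layers that move fully out of view destroy themselves and print their lifetime for debugging.
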(event Custom|InitLayer
  (params (SpeedCoef :type Float%20%28double-precision%29) (LayerMesh :type Static%20Mesh%20Object%20Reference) (bCanSpawnNewLayerRight :type Boolean) (bCanSpawnNewLayerLeft :type Boolean) (BgHolland :type BP%20Bg%20Holland%2001%20Object%20Reference))
  (Variables|Default|SetSpeedCoef SpeedCoef)
  (Variables|Default|SetLayerMesh LayerMesh)
  (Variables|Default|SetbCanSpawnNewLayerRight bCanSpawnNewLayerRight)
  (Variables|Default|SetbCanSpawnNewLayerLeft bCanSpawnNewLayerLeft)
  (Variables|Default|SetBgHolland BgHolland)
  (Components|StaticMesh|SetStaticMesh (Variables|Default|GetStaticMesh) (Variables|Default|GetLayerMesh)))

(event EventBeginPlay
  (bind _returnvalue (Game|Player|GetPlayerPawn 0))
  (Utilities|IsValid _returnvalue
    (:Is%20Valid
      (Variables|Default|SetLastCameraLocation (Transformation|GetActorLocation _returnvalue)))))

(event Collision|EventActorBeginOverlap
  (params (OtherActor :type Actor%20Object%20Reference)))

(event EventTick
  (params (DeltaSeconds :type Float%20%28single-precision%29))
  (bind _returnvalue (Game|Player|GetPlayerPawn 0))
  (bind _returnvalue_2 (Transformation|GetActorLocation))
  (bind _returnvalue_3 (Transformation|GetActorRotation))
  (bind _returnvalue_4 (Transformation|GetActorScale3D))
  (bind _self self)
  (bind _layermesh (Variables|Default|GetLayerMesh))
  (bind _speedcoef (Variables|Default|GetSpeedCoef))
  (bind _staticmesh (Variables|Default|GetStaticMesh))
  (bind _speedcoef_2 (Variables|Default|GetSpeedCoef))
  (bind _boxextent (Collision|GetComponentBounds _staticmesh))
  (bind _returnvalue_5 (Transformation|GetActorLocation _returnvalue))
  (bind _returnvalue_6 (Transformation|GetActorLocation _returnvalue))
  (bind _y (Math|Vector|BreakVector _boxextent))
  (bind _y_2 (Math|Vector|BreakVector _returnvalue_5))
  (bind _returnvalue_7 (+ (.y _returnvalue_2) _y))
  (bind _returnvalue_8 (- (.y _returnvalue_2) _y))
  (Variables|Default|SetLifeTimeDebug (+ (Variables|Default|GetLifeTimeDebug) DeltaSeconds))
  (Utilities|IsValid (Variables|Default|GetStaticMesh)
    (:Is%20Valid
      (Utilities|IsValid (Variables|Default|GetLayerMesh)
        (:Is%20Valid
          (Utilities|IsValid _returnvalue
            (:Is%20Valid
              (Transformation|AddActorWorldOffset (Math|Vector|MakeVector 0.0 (* _speedcoef (- (.y _returnvalue_6) (.y (Variables|Default|GetLastCameraLocation)))) (* _speedcoef (- (.z _returnvalue_6) (.z (Variables|Default|GetLastCameraLocation))))))
              (Variables|Default|SetLastCameraLocation _returnvalue_5)
              (bind _diagonale (CallFunction|FindDiagonalefromScreenPosition))
              (Utilities|FlowControl|Sequence
                (:then_0
                  (if (< (- _y_2 (Math|Float|Absolute(Float) (.Y (Math|Vector|BreakVector _diagonale)))) _returnvalue_8)
                    (Utilities|IsValid (Variables|Default|GetLeftLayer)
                      (:Is%20Not%20Valid
                        (bind _returnvalue_9 (Game|SpawnActorfromClass (Utilities|GetClass self) (Math|Transform|MakeTransform (+ (Transformation|GetActorLocation) (Math|Vector|MakeVector 0.0 (+ (* _y -2.0) 4e+01) 0.0)) _returnvalue_3 _returnvalue_4) "Undefined" "MultiplyWithRoot" 0 _speedcoef_2 _layermesh false true 0 _self 0 _self 0))
                        (Variables|Default|SetLeftLayer _returnvalue_9)))))
                (:then_1
                  (if (> (+ _y_2 (Math|Float|Absolute(Float) (.Y (Math|Vector|BreakVector _diagonale)))) _returnvalue_7)
                    (Utilities|IsValid (Variables|Default|GetRightLayer)
                      (:Is%20Not%20Valid
                        (bind _returnvalue_10 (Game|SpawnActorfromClass (Utilities|GetClass self) (Math|Transform|MakeTransform (+ (Transformation|GetActorLocation) (Math|Vector|MakeVector 0.0 (- (* _y 2.0) 4e+01) 0.0)) _returnvalue_3 _returnvalue_4) "Undefined" "MultiplyWithRoot" 0 _speedcoef_2 _layermesh true false 0 0 self _self 0))
                        (Variables|Default|SetRightLayer _returnvalue_10)))))
                (:then_2
                  (if (> (- _y_2 (Math|Float|Absolute(Float) (.Y (Math|Vector|BreakVector _diagonale)))) _returnvalue_7)
                    (Actor|DestroyActor)
                    (Development|PrintString (Utilities|String|ToString(Float) (Variables|Default|GetLifeTimeDebug)) :!label _label)))
                (:then_3
                  (if (< (+ _y_2 (Math|Float|Absolute(Float) (.Y (Math|Vector|BreakVector _diagonale)))) _returnvalue_8)
                    (Actor|DestroyActor)
                    (goto _label)))))))))))

(fn ConstructionScript
  (Components|StaticMesh|SetStaticMesh (Variables|Default|GetStaticMesh) (Variables|Default|GetLayerMesh)))

(fn FindDiagonalefromScreenPosition
  (params (ScreenPosition :type Vector%202D%20Structure))
  (bind _returnvalue (Game|Player|GetPlayerPawn 0))
  (bind _returnvalue_2 (Game|GetPlayerController 0))
  (bind (_worldposition _worlddirection) (Class|GameplayStatics|DeprojectScreentoWorld _returnvalue_2 ScreenPosition))
  (bind _returnvalue_3 (Transformation|GetActorLocation _returnvalue))
  (bind _returnvalue_4 (- _worldposition _returnvalue_3))
  (return (* (Math|Vector|Normalize (Math|Vector|MakeVector 0.0 (.y _returnvalue_4) (.z _returnvalue_4))) (* (Math|Trig|Tan(Radians) (Math|Trig|Acos(Degrees) (Math|Vector|DotProduct (Transformation|GetActorForwardVector _returnvalue) _worlddirection))) (- (.x (Transformation|GetActorLocation)) (.x (Transformation|GetActorLocation _returnvalue)))))))