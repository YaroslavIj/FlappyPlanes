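; Player controller that owns the match UI: the in-game HUD, pause menu, start timer and end-game screen.
; On BeginPlay the local controller creates the HUD, and events forward health, projectile count and fuel to its sub-widgets.
; Space opens the pause widget with UI-only input and pauses the game.
; Separate events show the start-game widget and a win-or-lose end screen with the mouse cursor visible.
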(event Custom|CreateStartGameTimer
  (bind _returnvalue (UserInterface|CreateWidget "/Game/Widgets/Game/BPW_StartGame.BPW_StartGame_C"))
  (UserInterface|Viewport|AddtoViewport _returnvalue 0))

(event Custom|SetHealthOnWidget
  (params (Health :type Float%20%28double-precision%29))
  (bind _ingamewidget (Variables|Default|GetInGameWidget))
  (Utilities|IsValid _ingamewidget
    (:Is%20Valid
      (Default|SetHealth (Variables|/Game/Widgets/Game/BPW_InGame.BPW_InGame_C|GetBPW_Health _ingamewidget) Health))))

(event Custom|SetProjectilesAmountOnWidgt
  (params (ProjectilesAmount :type Float%20%28double-precision%29))
  (bind _ingamewidget (Variables|Default|GetInGameWidget))
  (Utilities|IsValid _ingamewidget
    (:Is%20Valid
      (Default|SetProjectiles (Variables|/Game/Widgets/Game/BPW_InGame.BPW_InGame_C|GetBPW_Projectiles _ingamewidget) ProjectilesAmount))))

(event Custom|SetFuelOnWidget
  (params (Fuel :type Float%20%28double-precision%29))
  (bind _ingamewidget (Variables|Default|GetInGameWidget))
  (Utilities|IsValid _ingamewidget
    (:Is%20Valid
      (Default|SetFuel (Variables|/Game/Widgets/Game/BPW_InGame.BPW_InGame_C|GetBPW_Fuel _ingamewidget) Fuel))))

(event Custom|EndGame_Client
  (params (bIsWin :type Boolean))
  (bind _returnvalue (UserInterface|CreateWidget "/Game/Widgets/Game/BPW_EndGame.BPW_EndGame_C" 0 bIsWin))
  (UserInterface|Viewport|AddtoViewport _returnvalue 0)
  (Variables|Default|SetbShowMouseCursor true))

(event EventBeginPlay
  (if (Pawn|IsLocalController)
    (bind _returnvalue (UserInterface|CreateWidget "/Game/Widgets/Game/BPW_InGame.BPW_InGame_C"))
    (bind _output_get (Variables|Default|SetInGameWidget _returnvalue))
    (UserInterface|Viewport|AddtoViewport _output_get 0)))

(event EventTick
  (params (DeltaSeconds :type Float%20%28single-precision%29)))

(event Input|KeyboardEvents|SpaceBar
  (params (Key :type Key%20Structure :default "None"))
  (:Pressed
    (Variables|Default|SetbShowMouseCursor true)
    (bind _returnvalue (UserInterface|CreateWidget "/Game/Widgets/Game/BPW_Pause.BPW_Pause_C"))
    (UserInterface|Viewport|AddtoViewport _returnvalue 0)
    (Input|SetInputModeUIOnly self _returnvalue "DoNotLock" false)
    (Game|SetGamePaused true)))

(fn ConstructionScript)